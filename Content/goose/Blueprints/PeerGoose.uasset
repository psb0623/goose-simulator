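; Companion goose that joins the player's flock when the ThirdPersonCharacter overlaps it, with a preset that sets its material and can grant super-move or fireball items.
; Each Tick it takes delayed position and rotation from the character or preceding goose, buffering its own with alternating side offsets for the next follower.
; Missile shots ripple down the chain through the same delay buffers, while fire input launches bullets along the player's aim from each following goose.
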(event OnComponentBeginOverlap(Box)
  (params (OverlappedComponent :type Primitive%20Component%20Object%20Reference) (OtherActor :type Actor%20Object%20Reference) (OtherComp :type Primitive%20Component%20Object%20Reference) (OtherBodyIndex :type Integer) (bFromSweep :type Boolean) (SweepResult :type Hit%20Result%20Structure%20%28by%20ref%29))
  (bind _prevrotarr (Variables|Default|GetPrevRotArr))
  (bind _prevposarr (Variables|Default|GetPrevPosArr))
  (bind _presettype (Variables|Default|GetPresetType))
  (if (not (Variables|Default|GetIsFollowing))
    (bind _asthird_person_character (Utilities|Casting|CastToThirdPersonCharacter OtherActor))
    (Variables|Default|SetIsFollowing true)
    (bind _output_get (Variables|Default|Setorigin _asthird_person_character))
    (bind _output_get_2 (Variables|Default|SetPeerIdx (Utilities|Array|Length (Variables|/Game/goose/Blueprints/ThirdPersonCharacter.ThirdPersonCharacter_C|GetPeers _output_get))))
    (Utilities|Array|Add (Variables|/Game/goose/Blueprints/ThirdPersonCharacter.ThirdPersonCharacter_C|GetPeers _output_get) self)
    (Variables|Default|SetPrePeer (Utilities|Array|Get(acopy) (Variables|/Game/goose/Blueprints/ThirdPersonCharacter.ThirdPersonCharacter_C|GetPeers _output_get) (- _output_get_2 1)))
    (for _index (range 0 14)
      (Utilities|Array|Add _prevposarr (- (Transformation|GetWorldLocation (Variables|Default|Getgoose_lowpoly)) "0, 0, 0"))
      (Utilities|Array|Add _prevrotarr (Math|Rotator|GetRotationXVector (Transformation|GetWorldRotation (Variables|Default|Getgoose_lowpoly))))
      (Utilities|Array|Add (Variables|Default|GetPrevMissileArr) false))
    (Variables|Default|SetPrevPos (Utilities|Array|Get(acopy) _prevposarr))
    (Variables|Default|SetPrevRot (Utilities|Array|Get(acopy) _prevrotarr))
    (if (== _presettype 1)
      (Variables|/Game/goose/Blueprints/ThirdPersonCharacter.ThirdPersonCharacter_C|SetSuperMoveItem (Variables|Default|Getorigin) true)
      (Effects|SpawnEmitterAttached "/Game/goose/Blueprints/SuperMove.SuperMove" (Variables|/Game/goose/Blueprints/ThirdPersonCharacter.ThirdPersonCharacter_C|Getgoose (Variables|Default|Getorigin)) "None" "0, 0, 0" "90.000000,0.000000,90.000000" "6.000000,6.000000,6.000000")
      (elif (== _presettype 2)
        (Variables|/Game/goose/Blueprints/ThirdPersonCharacter.ThirdPersonCharacter_C|SetFireBallItem (Variables|Default|Getorigin) true)))))

(event EventBeginPlay
  (Input|EnableInput (Game|GetPlayerController 0))
  (switch int (Variables|Default|GetPresetType)
    (:Default
      (Rendering|Material|SetMaterial (Variables|Default|Getgoose_lowpoly) 0 "/Game/goose/Material_001.Material_001" :!label _label))
    (:0
      (goto _label))
    (:1
      (Rendering|Material|SetMaterial (Variables|Default|Getgoose_lowpoly) 0 "/Game/StarterContent/Materials/M_Tech_Hex_Tile_Pulse.M_Tech_Hex_Tile_Pulse"))
    (:2
      (Rendering|Material|SetMaterial (Variables|Default|Getgoose_lowpoly) 0 "/Game/STF/Pack03-LandscapePro/Environment/Landscape/Landscape/v2/MI_landscape_pro_v2_no_tesselation_Inst.MI_landscape_pro_v2_no_tesselation_Inst"))))

(event Collision|EventActorBeginOverlap
  (params (OtherActor :type Actor%20Object%20Reference)))

(event EventTick
  (params (DeltaSeconds :type Float%20%28single-precision%29))
  (bind _origin (Variables|Default|Getorigin))
  (bind _prevrotarr (Variables|Default|GetPrevRotArr))
  (bind _prevposarr (Variables|Default|GetPrevPosArr))
  (bind _prevmissilearr (Variables|Default|GetPrevMissileArr))
  (bind _prevmissilearr_2 (Variables|Default|GetPrevMissileArr))
  (bind _origin_2 (Variables|Default|Getorigin))
  (bind _peeridx (Variables|Default|GetPeerIdx))
  (bind _bulletoffset (Variables|Default|GetBulletOffset))
  (bind _goose_lowpoly (Variables|Default|Getgoose_lowpoly))
  (bind _returnvalue (Transformation|GetWorldLocation _goose_lowpoly))
  (bind _returnvalue_2 (+ _peeridx 1))
  (bind _prevmissilearr_3 (Variables|/Game/goose/Blueprints/ThirdPersonCharacter.ThirdPersonCharacter_C|GetPrevMissileArr _origin))
  (bind _missiletransform (Variables|/Game/goose/Blueprints/ThirdPersonCharacter.ThirdPersonCharacter_C|GetMissileTransform _origin_2))
  (bind _missileimpulsedir (Variables|/Game/goose/Blueprints/ThirdPersonCharacter.ThirdPersonCharacter_C|GetMissileImpulseDir _origin_2))
  (bind _returnvalue_3 (Math|Vector|RotateVector _bulletoffset _missiletransform))
  (bind _returnvalue_4 (Math|Conversions|ToFloat(Integer) _returnvalue_2))
  (bind _output (Utilities|Array|Get(acopy) _prevmissilearr_3))
  (bind _returnvalue_5 (+ _returnvalue _returnvalue_3))
  (bind _returnvalue_6 (Math|Transform|MakeTransform _returnvalue_5 _missiletransform))
  (if (Variables|Default|GetIsFollowing)
    (Utilities|Array|Add _prevposarr (+ (Transformation|GetWorldLocation (Variables|Default|Getgoose_lowpoly)) (Math|Vector|RotateVector (Math|Vector|MakeVector (* (Math|Float|Power -1.0 _returnvalue_4) _returnvalue_4 (Math|Trig|Cos(Degrees) (Variables|Default|Gettheta)) (Variables|Default|Getdistance)) (Math|Float|Min(Float) (* (Math|Trig|Sin(Degrees) (Variables|Default|Gettheta)) (Variables|Default|Getdistance) (Math|Float|Power -1.0 _returnvalue_4)) 0.0) 0.0) (Math|Conversions|RotationFromXVector (Variables|/Game/goose/Blueprints/ThirdPersonCharacter.ThirdPersonCharacter_C|GetCamOffset (Variables|Default|Getorigin))))))
    (Utilities|Array|RemoveIndex _prevposarr)
    (Variables|Default|SetPrevPos (Utilities|Array|Get(acopy) _prevposarr))
    (Utilities|Array|Add _prevrotarr (Math|Rotator|GetRotationXVector (Transformation|GetWorldRotation (Variables|Default|Getgoose_lowpoly))))
    (Utilities|Array|RemoveIndex _prevrotarr)
    (Variables|Default|SetPrevRot (Utilities|Array|Get(acopy) _prevrotarr))
    (if (Variables|Default|GetSuperMoveItem)
      _
      (elif (Variables|/Game/goose/Blueprints/ThirdPersonCharacter.ThirdPersonCharacter_C|GetSuperMoveItem (Variables|Default|Getorigin))
        (Effects|SpawnEmitterAttached "/Game/goose/Blueprints/SuperMove.SuperMove" (Variables|Default|Getgoose_lowpoly) "None" "0, 0, 0" "90.000000,0.000000,90.000000" "6.000000,6.000000,6.000000")
        (Variables|Default|SetSuperMoveItem true)))
    (if (<= (Variables|Default|GetPeerIdx) 1)
      (Transformation|SetWorldLocation (Variables|Default|Getgoose_lowpoly) (Variables|/Game/goose/Blueprints/ThirdPersonCharacter.ThirdPersonCharacter_C|GetPrevPos _origin) false false)
      (Transformation|SetWorldRotation (Variables|Default|Getgoose_lowpoly) (Math|Conversions|RotationFromXVector (Variables|/Game/goose/Blueprints/ThirdPersonCharacter.ThirdPersonCharacter_C|GetPrevRot _origin)) false false)
      (if _output
        (bind _returnvalue_7 (Game|SpawnActorfromClass "/Game/VigilanteContent/Projectiles/West_Missile_M26/missile.missile_C" _returnvalue_6 "AdjustIfPossibleButAlwaysSpawn" 0 0))
        (Physics|AddImpulse (Variables|/Game/VigilanteContent/Projectiles/West_Missile_M26/missile.missile_C|GetSphere _returnvalue_7) _missileimpulsedir "None" false))
      (Utilities|Array|Add _prevmissilearr_2 _output)
      (Utilities|Array|RemoveIndex _prevmissilearr_2)
      (else
        (bind _aspeer_goose (Utilities|Casting|CastToPeerGoose (Variables|Default|GetPrePeer)))
        (Transformation|SetWorldLocation (Variables|Default|Getgoose_lowpoly) (Variables|PeerGoose_C|GetPrevPos _aspeer_goose) false false)
        (Transformation|SetWorldRotation (Variables|Default|Getgoose_lowpoly) (Math|Conversions|RotationFromXVector (Variables|PeerGoose_C|GetPrevRot _aspeer_goose)) false false)
        (if (Utilities|Array|Get(acopy) (Variables|PeerGoose_C|GetPrevMissileArr _aspeer_goose))
          (bind _returnvalue_8 (Game|SpawnActorfromClass "/Game/VigilanteContent/Projectiles/West_Missile_M26/missile.missile_C" _returnvalue_6 "AdjustIfPossibleButAlwaysSpawn" 0 0))
          (Physics|AddImpulse (Variables|/Game/VigilanteContent/Projectiles/West_Missile_M26/missile.missile_C|GetSphere _returnvalue_8) _missileimpulsedir "None" false))
        (Utilities|Array|Add _prevmissilearr (Utilities|Array|Get(acopy) (Variables|PeerGoose_C|GetPrevMissileArr _aspeer_goose)))
        (Utilities|Array|RemoveIndex _prevmissilearr)))))

(event Input|ActionEvents|InputActionfire
  (params (Key :type Key%20Structure :default "None"))
  (bind _returnvalue (Game|Player|GetPlayerPawn 0))
  (bind _returnvalue_2 (Pawn|GetControlRotation _returnvalue :!class /Script/Engine.Pawn))
  (bind _returnvalue_3 (Math|Rotator|GetRotationXVector _returnvalue_2))
  (:Pressed
    (if (Variables|Default|GetIsFollowing)
      (bind _returnvalue_4 (Game|SpawnActorfromClass "/Game/goose/Blueprints/Bullet.Bullet_C" (Math|Conversions|ToTransform(Vector) (+ (Transformation|GetWorldLocation (Variables|Default|Getgoose_lowpoly)) (* _returnvalue_3 1e+02))) "Undefined" 0 0))
      (Physics|AddImpulse (Variables|/Game/goose/Blueprints/Bullet.Bullet_C|GetSphere _returnvalue_4) (* _returnvalue_3 1e+04) "None" true))))

(fn ConstructionScript)