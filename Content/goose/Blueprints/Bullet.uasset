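; Bullet is a projectile actor that damages the BossAI enemy on impact.
; It attaches a particle effect to its sphere on spawn and destroys itself once a Tick-driven timer expires.
; Hits on anything except itself and the ThirdPersonCharacter spawn an explosion and destroy the bullet.
; A BossAI hit subtracts fixed HP, and at zero it ragdolls the boss, disables capsule collision and stops its AI brain logic.
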(event OnComponentBeginOverlap(Sphere)
  (params (OverlappedComponent :type Primitive%20Component%20Object%20Reference) (OtherActor :type Actor%20Object%20Reference) (OtherComp :type Primitive%20Component%20Object%20Reference) (OtherBodyIndex :type Integer) (bFromSweep :type Boolean) (SweepResult :type Hit%20Result%20Structure%20%28by%20ref%29)))

(event EventBeginPlay
  (Effects|SpawnEmitterAttached "/Game/StarterContent/Particles/P_Explosion_3.P_Explosion_3" (Variables|Default|GetSphere) "None"))

(event Collision|EventActorBeginOverlap
  (params (OtherActor :type Actor%20Object%20Reference)))

(event EventTick
  (params (DeltaSeconds :type Float%20%28single-precision%29))
  (bind _output_get (Variables|Default|SetTimeElapsed (+ DeltaSeconds (Variables|Default|GetTimeElapsed))))
  (if (<= 6.0 _output_get)
    (Actor|DestroyActor)))

(event Collision|EventHit
  (params (MyComp :type Primitive%20Component%20Object%20Reference) (Other :type Actor%20Object%20Reference) (OtherComp :type Primitive%20Component%20Object%20Reference) (bSelfMoved :type Boolean) (HitLocation :type Vector :default "0, 0, 0") (HitNormal :type Vector :default "0, 0, 0") (NormalImpulse :type Vector :default "0, 0, 0") (Hit :type Hit%20Result%20Structure%20%28by%20ref%29))
  (bind _returnvalue (Actor|GetActorOfClass "/Game/goose/Blueprints/ThirdPersonCharacter.ThirdPersonCharacter_C"))
  (if (and (!= self Other) (!= Other _returnvalue))
    (Effects|SpawnEmitteratLocation "/Game/StarterContent/Particles/P_Explosion_4.P_Explosion_4" HitLocation "0, 0, 0" "2.000000,2.000000,2.000000")
    (Actor|DestroyActor)
    (bind _asboss_ai (Utilities|Casting|CastToBossAI Other))
    (bind _output_get (Variables|/Game/enemy/BossAI.BossAI_C|SetHP _asboss_ai (- (Variables|/Game/enemy/BossAI.BossAI_C|GetHP _asboss_ai) 1e+02)))
    (if (<= _output_get 0.0)
      (Physics|SetSimulatePhysics (Variables|/Script/Engine.Character|GetMesh _asboss_ai) true)
      (Collision|SetCollisionEnabled (Variables|/Script/Engine.Character|GetCapsuleComponent _asboss_ai) "NoCollision")
      (AI|Logic|StopLogic (Variables|/Script/AIModule.AIController|GetBrainComponent (AI|GetAIController _asboss_ai)) "")
      (else
        (Development|PrintString (Utilities|String|ToString(Float) _output_get))))))

(fn ConstructionScript)